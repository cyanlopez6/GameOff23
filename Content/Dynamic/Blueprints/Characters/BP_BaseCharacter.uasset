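; Base character Blueprint that manages hit points and walk speed, initializing both at BeginPlay.
; Damage clamps health, applies knockback away from the source and starts timed invincibility.
; Max HP changes cap current HP, with increases routed through the damage event, so they also trigger or are blocked by invincibility.
; Speed changes accumulate in a modifier subtracted from the default, so a positive "reduction" actually raises speed.
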(event `self.ReceiveBeginPlay`
  (set `CharacterMovementComponent.MaxWalkSpeed` (`self.Default Walk Speed`) (`self.CharacterMovement`))
  (set `self.Current Hit Points` (`self.Max Hit Points`)))

(event `/Game/Dynamic/Blueprints/Characters/BPI_BaseCharacter.Reduce Max Walk Speed`
  (params (`Reduction Amount` :type "Float (double-precision)"))
  ;[1 1 1] Reduce the movement speed of the character and keep track of how much the speed has been reduced.
  (bind _output_get (set `self.Walk Speed Modifier` (- (`self.Walk Speed Modifier`) `Reduction Amount`)))
  (set `CharacterMovementComponent.MaxWalkSpeed` (- (`self.Default Walk Speed`) _output_get) (`self.CharacterMovement`)))

(event `/Game/Dynamic/Blueprints/Characters/BPI_BaseCharacter.Reduce Current Hit Points`
  (params (`Reduction Amount` :type "Float (double-precision)") (`Damage Source Location` :type "Vector Structure") (`Damage Knock Back` :type "Float (double-precision)"))
  ;[1 1 1] Reduce Current HP by specified amount, clamping between 0 and Max HP
  (if (not (`self.Invincible`))
    (set `self.Current Hit Points` (`KismetMathLibrary.FClamp` (- (`self.Current Hit Points`) `Reduction Amount`) 0.0 (`self.Max Hit Points`)))
    ;[1 1 1] Create Knockback that goes away from the damage source
    (`CharacterMovementComponent.AddImpulse` (`self.CharacterMovement`) (* (- (`self.K2_GetActorLocation`) `Damage Source Location`) `Damage Knock Back`) false)
    ;[1 1 1] Grant temporary invincibility when character takes damage
    (bind _returnvalue (`KismetSystemLibrary.K2_SetTimerDelegate` (delegate `Invincibility Stopped`) (`self.Invincibility Time`)))
    (set `self.Invincibility Timer` _returnvalue)
    (set `self.Invincible` true)))

(event `Invincibility Stopped`
  ;[1 1 1] Grant temporary invincibility when character takes damage
  (set `self.Invincible` false))

(event `/Game/Dynamic/Blueprints/Characters/BPI_BaseCharacter.Reduce Max Hit Points`
  (params (`Reduction Amount` :type "Float (double-precision)"))
  ;[1 1 1] Reduce Max HP by the specified amount
  (bind _output_get (set `self.Max Hit Points` (- (`self.Max Hit Points`) `Reduction Amount`)))
  (if (< _output_get (`self.Current Hit Points`))
    ;[1 1 1] If Max HP < Current HP, set it to current HP
    (set `self.Current Hit Points` (`self.Max Hit Points`))
    (else
      ;[1 1 1] Reduction by a negative results in an increase in health. Increase Current HP by equal amount
      (if (< (`KismetMathLibrary.SignOfFloat` `Reduction Amount`) 0.0)
        (`/Game/Dynamic/Blueprints/Characters/BPI_BaseCharacter.Reduce Current Hit Points` `Reduction Amount`)))))

(fn `UserConstructionScript`)