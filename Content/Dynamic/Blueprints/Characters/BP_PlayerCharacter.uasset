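; Player character Blueprint with Enhanced Input for jumping and movement along the world X axis.
; Timers add jump forgiveness: a jump buffer re-triggers Jump on landing, and a CanJumpInternal override allows coyote-time jumps after falling.
; Jumping clears both timers.
; Helper functions adjust hit points and walk speed, though ReduceCurrentHitPoints writes its clamped result to MaxHitPoints instead of CurrentHitPoints.
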(event `self.ReceiveBeginPlay`
  (`self.Apply Input Mapping Context`)
  (set `CharacterMovementComponent.MaxWalkSpeed` (`self.Default Walk Speed`) (`self.CharacterMovement`)))

(event `EnhancedInput|/Game/Dynamic/Blueprints/Characters/Inputs/IA_Jump`
  (params (ActionValue :type Boolean) (ElapsedSeconds :type "Float (double-precision)") (TriggeredSeconds :type "Float (double-precision)") (InputAction :type "InputAction Object Reference" :default "/Game/Dynamic/Blueprints/Characters/Inputs/IA_Jump.IA_Jump"))
  ;[1 1 1] Handle Inputs
  (:`Triggered`
    (`self.Jump`)
    ;[1 1 1] Jump Buffer, which lets player hit jump slightly before landing to jump when landing
    (bind _returnvalue (`KismetSystemLibrary.K2_SetTimerDelegate` (delegate `Jump Buffer Ended`) (`self.Jump Buffer Time`)))
    (set `self.Jump Buffer Timer` _returnvalue))
  (:`Completed`
    (`self.StopJumping`)))

(event `Jump Buffer Ended`
  ;[1 1 1] Jump Buffer, which lets player hit jump slightly before landing to jump when landing
)

(event `EnhancedInput|/Game/Dynamic/Blueprints/Characters/Inputs/IA_MoveRight`
  (params (ActionValue :type "Float (double-precision)") (ElapsedSeconds :type "Float (double-precision)") (TriggeredSeconds :type "Float (double-precision)") (InputAction :type "InputAction Object Reference" :default "/Game/Dynamic/Blueprints/Characters/Inputs/IA_MoveRight.IA_MoveRight"))
  ;[1 1 1] Handle Inputs
  (:`Triggered`
    (`self.AddMovementInput` (1.0 0.0 0.0) ActionValue)))

(event `self.K2_OnMovementModeChanged`
  (params (PrevMovementMode :type "EMovementMode Enum" :default "MOVE_None") (NewMovementMode :type "EMovementMode Enum" :default "MOVE_None") (PrevCustomMode :type Byte) (NewCustomMode :type Byte))
  ;[1 1 1] Add Coyote Time delay when falling off of a ledge. This allows player to jump slightly after they fall off of a ledge
  (if (and (not (`KismetSystemLibrary.K2_IsValidTimerHandle` (`self.Coyote Timer`))) (`|EnumEquality` NewMovementMode "MOVE_Falling"))
    (bind _returnvalue (`KismetSystemLibrary.K2_SetTimerDelegate` (delegate `CoyoteTimeEnded`) (`self.Coyote Time`)))
    (set `self.Coyote Timer` _returnvalue)))

(event `CoyoteTimeEnded`
  ;[1 1 1] Add Coyote Time delay when falling off of a ledge. This allows player to jump slightly after they fall off of a ledge
)

(event `self.OnJumped`
  ;[1 1 1] Add Coyote Time delay when falling off of a ledge. This allows player to jump slightly after they fall off of a ledge
  (`KismetSystemLibrary.K2_ClearAndInvalidateTimerHandle` (`self.Coyote Timer`))
  (`KismetSystemLibrary.K2_ClearAndInvalidateTimerHandle` (`self.Jump Buffer Timer`)))

(event `self.OnLanded`
  (params (Hit :type "HitResult Structure (by ref)"))
  ;[1 1 1] When Landing, reset Coyote Time and jump if the Jump Buffer is still active
  (`KismetSystemLibrary.K2_ClearAndInvalidateTimerHandle` (`self.Coyote Timer`))
  (if (> (`KismetSystemLibrary.K2_GetTimerRemainingTimeHandle` (`self.Jump Buffer Timer`)) 0.0)
    (`self.Jump`)
    (`KismetSystemLibrary.K2_ClearAndInvalidateTimerHandle` (`self.Jump Buffer Timer`))))

(fn `Apply Input Mapping Context`
  (bind _asplayer_controller (cast `PlayerController` (`self.GetController`)))
  (bind _returnvalue (pcsubsystem `EnhancedInputLocalPlayerSubsystem` _asplayer_controller))
  (`/Engine/EditorBlueprintResources/StandardMacros.IsValid` _returnvalue
    (:`Is Valid`
      (`EnhancedInputSubsystemInterface.AddMappingContext` _returnvalue "/Game/Dynamic/Blueprints/Characters/Inputs/IM_PlayerInputMapping.IM_PlayerInputMapping" 0 (struct)))))

(fn `CanJumpInternal`
  (returns (ReturnValue :type Boolean))
  ;[1 1 1] Allow normal jump or a coyote time jump
  (bind _returnvalue (`parent.CanJumpInternal`))
  (return (or _returnvalue (> (`KismetSystemLibrary.K2_GetTimerRemainingTimeHandle` (`self.Coyote Timer`)) 0.0))))

(fn `Reduce Current Hit Points`
  (params (`Reduction Amount` :type "Float (double-precision)"))
  ;[1 1 1] Reduce Current HP by specified amount, clamping between 0 and Max HP
  (set `self.Max Hit Points` (`KismetMathLibrary.FClamp` (- (`self.Current Hit Points`) `Reduction Amount`) 0.0 (`self.Max Hit Points`))))

(fn `Reduce Max Hit Points`
  (params (`Reduction Amount` :type "Float (double-precision)"))
  ;[1 1 1] Reduce Max HP by the specified amount
  (bind _output_get (set `self.Max Hit Points` (- (`self.Max Hit Points`) `Reduction Amount`)))
  (if (< _output_get (`self.Current Hit Points`))
    ;[1 1 1] If Max HP < Current HP, set it to current HP
    (set `self.Current Hit Points` (`self.Max Hit Points`))
    (else
      ;[1 1 1] Reduction by a negative results in an increase in health. Increase Current HP by equal amount
      (if (< (`KismetMathLibrary.SignOfFloat` `Reduction Amount`) 0.0)
        (`self.Reduce Current Hit Points` `Reduction Amount`)))))

(fn `Reduce Max Walk Speed`
  (params (`Reduction Amount` :type "Float (double-precision)"))
  ;[1 1 1] Reduce the movement speed of the character and keep track of how much the speed has been reduced.
  (bind _output_get (set `self.Walk Speed Modifier` (- (`self.Walk Speed Modifier`) `Reduction Amount`)))
  (set `CharacterMovementComponent.MaxWalkSpeed` (- (`self.Default Walk Speed`) _output_get) (`self.CharacterMovement`)))

(fn `UserConstructionScript`)